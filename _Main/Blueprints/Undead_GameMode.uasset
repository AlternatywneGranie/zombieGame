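; Game mode for a wave-based zombie survival game, handling spawning, wave progression, and win and lose screens.
; On BeginPlay it spawns a zombie count scaled by the current wave, split between two spawn locations.
; ZombieKilled counts down the remainder; at zero, the next wave shows its UI and spawns after a delay, or the player wins if on the final wave.
; Win, lose and wave UI go through BP_FirstPersonCharacter.
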(event `self.ReceiveBeginPlay`
  ;[1 0.1491 0.8648] Start Game
  (`self.Start Game`))

(event `Start Game`
  ;[1 0.1491 0.8648] Start Game
  (`self.Spawn Zombies`))

(event `Spawn Zombies`
  ;[0.4247 1 0.5967] Spawn Zombies
  (bind _output_get (set `self.ZombieTotal` (* (`self.CurrentWave`) 8)))
  (set `self.ZombiesLeft` _output_get)
  (for _index (range (+ _output_get 1))
    (if (== _index (/ (`self.ZombieTotal`) 2))
      (break)
      (else
        (`|SpawnActorFromClass` "/Game/_Main/Zombie/BP_Zombie.BP_Zombie_C" (`self.SpawnLocation1`) "Undefined" "MultiplyWithRoot" null null))))
  (for _ (range 1 (+ (/ (`self.ZombieTotal`) 2) 1))
    (`|SpawnActorFromClass` "/Game/_Main/Zombie/BP_Zombie.BP_Zombie_C" (`self.SpawnLocation2`) "Undefined" "MultiplyWithRoot" null null)))

(event `Zombie Killed`
  ;[1 1 1] Zombie Killed
  (bind _result (`/Engine/EditorBlueprintResources/StandardMacros.DecrementInt` (`self.ZombiesLeft`))
    (:`  `
      (if (== _result 0)
        (`self.WaveIncrement`)))))

(event `WaveIncrement`
  ;[1 0.2033 0.7586] Waves logic
  (if (== (`self.CurrentWave`) (`self.MaxWaves`))
    (`self.PlayerWins`)
    (else
      (`/Engine/EditorBlueprintResources/StandardMacros.IncrementInt` (`self.CurrentWave`)
        (:`  `
          (`self.WaveStart`))))))

(event `WaveStart`
  ;[0 0.9759 1] Start Next Wave
  (bind _asbp_first_person_character (cast `/Game/_Main/Blueprints/BP_FirstPersonCharacter` (`GameplayStatics.GetPlayerCharacter` 0)))
  (`/Game/_Main/Blueprints/BP_FirstPersonCharacter.ShowWavesUI` _asbp_first_person_character (`self.CurrentWave`))
  (`KismetSystemLibrary.Delay` 5.0)
  (`self.Spawn Zombies`))

(event `PlayerWins`
  ;[0 0.25 1] Win Logic
  (bind _asbp_first_person_character (cast `/Game/_Main/Blueprints/BP_FirstPersonCharacter` (`GameplayStatics.GetPlayerCharacter` 0)))
  (`/Game/_Main/Blueprints/BP_FirstPersonCharacter.ShowWinUI` _asbp_first_person_character))

(event `PlayerLose`
  (bind _asbp_first_person_character (cast `/Game/_Main/Blueprints/BP_FirstPersonCharacter` (`GameplayStatics.GetPlayerCharacter` 0)))
  (`/Game/_Main/Widgets/Main_Widget_W.showDeathWindow` (`/Game/_Main/Blueprints/BP_FirstPersonCharacter.MainWidgetReference` _asbp_first_person_character)))

(fn `UserConstructionScript`)