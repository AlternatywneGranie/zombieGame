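; BP_Zombie is an enemy zombie that chases the player, attacks in melee and dies from point damage.
; An AIMoveTo loop leads into an attack montage, whose notify applies damage through a sphere overlap, and seeing a pawn sets walk speed.
; Damage plays a hit reaction or a random death montage, both loosening collision.
; Death also reports the kill to Undead_GameMode, then destroys the actor after a delay.
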(event `Death`
  (bind _zombiedeathanims (`self.ZombieDeathAnims`))
  ;[0 1 0.9174] ZombiesDeath
  (set `self.isDead?` true)
  (`MovementComponent.StopMovementImmediately` (`self.CharacterMovement`))
  (`|PlayMontage` (`self.Mesh`) (`|GetArrayItem` _zombiedeathanims (`KismetMathLibrary.RandomInteger` (`KismetArrayLibrary.Array_Length` _zombiedeathanims)))
    (:`then`
      (`PrimitiveComponent.SetCollisionResponseToChannel` (`self.CapsuleComponent`) "ECC_Pawn" "ECR_Overlap")
      (`PrimitiveComponent.SetCollisionEnabled` (`self.Mesh`) "NoCollision")
      (bind _asundead_game_mode (cast `/Game/_Main/Blueprints/Undead_GameMode` (`GameplayStatics.GetGameMode`)))
      (`/Game/_Main/Blueprints/Undead_GameMode.Zombie Killed` _asundead_game_mode)
      (`KismetSystemLibrary.Delay` 2.5)
      (`self.K2_DestroyActor`))))

(event `self.ReceivePointDamage`
  (params (Damage :type "Float (single-precision)") (DamageType :type "DamageType Object Reference") (HitLocation :type "Vector Structure") (HitNormal :type "Vector Structure") (HitComponent :type "PrimitiveComponent Object Reference") (BoneName :type Name) (ShotFromDirection :type "Vector Structure") (InstigatedBy :type "Controller Object Reference") (DamageCauser :type "Actor Object Reference") (HitInfo :type "HitResult Structure (by ref)"))
  ;[1 0 0] Health_Zombie
  (if (`self.isDead?`)
    _
    (elif (<= (`self.Health`) 0.0)
      (`self.Death`)
      (else
        (bind _output_get (set `self.Health` (- (`self.Health`) Damage)))
        (if (<= _output_get 0.0)
          (`self.Death`)
          (else
            (`|PlayMontage` (`self.Mesh`) "/Game/_Main/Zombie/Animations/hitReaction_Zombie.hitReaction_Zombie"
              (:`then`
                (`PrimitiveComponent.SetCollisionResponseToChannel` (`self.CapsuleComponent`) "ECC_Pawn" "ECR_Overlap")
                (`PrimitiveComponent.SetCollisionEnabled` (`self.Mesh`) "NoCollision")))))))))

(event `self.ReceiveBeginPlay`
  ;[1 0 0.9467] Chasing Player
  (`self.RunToPlayer`))

(event `RunToPlayer`
  ;[1 0.9126 0] Run/attack Player
  (if (not (`self.isDead?`))
    (`|AIMoveTo` self (0.0 0.0 0.0) (`GameplayStatics.GetPlayerController` 0) 40.0
      (:`OnSuccess`
        (`self.AttackPlayer`))
      (:`OnFail`
        (`self.RunToPlayer`)))))

(event `self.PawnSensing.OnSeePawn`
  (params (Pawn :type "Pawn Object Reference"))
  ;[1 0.6588 0.9928] Speed
  (set `CharacterMovementComponent.MaxWalkSpeed` 360.0 (`self.CharacterMovement`)))

(event `AttackPlayer`
  ;[0.03433 1 0.6214] attack player
  (`|PlayMontage` (`self.Mesh`) "/Game/_Main/Zombie/Animations/zombieAttack.zombieAttack"
    (:`OnCompleted`
      (`self.RunToPlayer`))
    (:`OnNotifyBegin`
      (`GameplayStatics.PlaySoundAtLocation` "/Game/_Main/Zombie/Sounds/atakkju.atakkju" (`self.K2_GetActorLocation`) (struct) 1.0 1.0 0.0 "/Game/MilitaryWeapSilver/Sound/Attenuation/WeaponShot_att.WeaponShot_att" null null null)
      (bind _outactors (`KismetSystemLibrary.SphereOverlapActors` (`SceneComponent.K2_GetComponentLocation` (`self.Arrow1`)) 80.0 (`|MakeArray` "ObjectTypeQuery3" :!type "EObjectTypeQuery Enum") "/Game/_Main/Blueprints/BP_FirstPersonCharacter.BP_FirstPersonCharacter_C" (`|MakeArray` self :!type "Actor Object Reference")))
      (if true
        (for _array_element _outactors
          (`GameplayStatics.ApplyDamage` _array_element 30.0 (`self.GetController`) self "/Script/Engine.DamageType"))))))

(fn `UserConstructionScript`)